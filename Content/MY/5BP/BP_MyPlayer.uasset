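; Player character Blueprint with left/right movement along the world X axis and jumping.
; Coin pickups and HP loss are forwarded through GetCoin and LoseHp event calls.
; BeginPlay replaces mesh materials with dynamic instances, which SetMeshColors tints through the TexColor parameter.
; Entering water sets IsWet, costs HP and turns the mesh blue, while leaving clears the flag and restores white.
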(event Custom|OnGetCoin
  (params (CoinValue :type Integer))
  (Default|CallGetCoinEvent CoinValue))

(event Custom|OnLoseHP
  (Default|CallLoseHpEvent))

(event Custom|OnIntoWater
  ;[1 1 1] 물에 빠질 때 파랗게 만들기
  (Utilities|FlowControl|Sequence
    (:then_0
      (Variables|Default|SetIsWet true))
    (:then_1
      (CallFunction|OnLoseHP))
    (:then_2
      (CallFunction|SetMeshColors "(R=0.007224,G=0.000000,B=1.000000,A=1.000000)"))))

(event Custom|OnOutWater
  ;[1 1 1] 물에 빠질 때 파랗게 만들기
  ;;[0.5718 1 0.9701] 물 밖에 나오면 다시 하얗게
  (Utilities|FlowControl|Sequence
    (:then_0
      (Variables|Default|SetIsWet false))
    (:then_1
      (CallFunction|SetMeshColors "(R=1.000000,G=1.000000,B=1.000000,A=1.000000)"))))

(event EventBeginPlay
  ;[1 1 1] 물에 빠질 때 파랗게 만들기
  (for (_array_element _array_index) (Rendering|Material|GetMaterials (Variables|Character|GetMesh))
    (bind _returnvalue (Rendering|Material|CreateDynamicMaterialInstance _array_element "None" :!class /Script/Engine.KismetMaterialLibrary))
    (Utilities|FlowControl|Sequence
      (:then_0
        (Utilities|Array|Insert (Variables|Default|GetMaterials) _returnvalue _array_index))
      (:then_1
        (Rendering|Material|SetMaterial (Variables|Character|GetMesh) _array_index _returnvalue)))))

(event Input|ActionEvents|InputActionJump
  (params (Key :type Key%20Structure :default "None"))
  (:Pressed
    (Character|Jump)))

(event Input|AxisEvents|InputAxisMoveLeft
  (params (AxisValue :type Float%20%28single-precision%29))
  ;[1 1 1] 왼쪽으로 이동
  (Pawn|Input|AddMovementInput (Math|Vector|MakeVector (Variables|Default|GetSpeed) 0.0 0.0) AxisValue false))

(event Input|AxisEvents|InputAxisMoveRight
  (params (AxisValue :type Float%20%28single-precision%29))
  ;[1 1 1] 오른쪽으로 이동
  (Pawn|Input|AddMovementInput (Math|Vector|MakeVector (Variables|Default|GetSpeed) 0.0 0.0) AxisValue false))

(fn ConstructionScript)

(fn SetMeshColors
  (params (Color :type Linear%20Color%20Structure))
  (for _array_element (Variables|Default|GetMaterials)
    (Rendering|Material|SetVectorParameterValue _array_element "TexColor" Color :!class /Script/Engine.MaterialInstanceDynamic)))