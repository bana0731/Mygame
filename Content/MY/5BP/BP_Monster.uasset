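; BP_Monster is a simple patrolling monster that wanders along the X axis and removes itself on death.
; Tick runs an Idle, Walk and Die state machine: Idle waits, then picks a random X target between walk bounds.
; Walk steps by Speed per frame while easing rotation toward the target, returning to Idle within a speed-derived distance set in the construction script.
; Die delays for the death animation time, then destroys the actor.
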(event EventBeginPlay)

(event Collision|EventActorBeginOverlap
  (params (OtherActor :type Actor%20Object%20Reference)))

(event EventTick
  (params (DeltaSeconds :type Float%20%28single-precision%29))
  (bind _returnvalue (Transformation|GetActorLocation))
  (switch Utilities|FlowControl|Switch|SwitchonBPE_MonsterState (Variables|Default|GetCurState)
    (:NewEnumerator0
      ;[1 1 1] Idle
      (Utilities|FlowControl|Delay (Variables|Default|GetWaitingTime))
      (Variables|Default|SetTargetPos (Math|Vector|MakeVector (Math|Random|RandomFloatinRange (Variables|Default|GetWalkStartXPos) (Variables|Default|GetWalkEndXPos)) (.y _returnvalue) (.z _returnvalue)))
      (Variables|Default|SetCurState "NewEnumerator1"))
    (:NewEnumerator1
      ;[1 1 1] 걷기
      (if (< (Math|Vector|Distance(Vector) (Variables|Default|GetTargetPos) (Transformation|GetActorLocation)) (Variables|Default|GetCheckCloseTarget))
        (Variables|Default|SetCurState "NewEnumerator0")
        (else
          (Transformation|SetActorLocationAndRotation (+ (* (Math|Vector|Normalize (Math|Vector|MakeVector (.X (Math|Vector|BreakVector (- (Variables|Default|GetTargetPos) (Transformation|GetActorLocation)))) 0.0 0.0)) (Variables|Default|GetSpeed)) (Transformation|GetActorLocation)) (Math|Rotator|Lerp(Rotator) (Transformation|GetActorRotation) (Math|Rotator|FindLookatRotation (Transformation|GetActorLocation) (Variables|Default|GetTargetPos)) 0.1)))))
    (:NewEnumerator2
      ;[1 1 1] 죽음
      (Utilities|FlowControl|Delay (Variables|Default|GetDieAniTime))
      (Actor|DestroyActor))))

(fn ConstructionScript
  ;[1 1 1] 몬스터 초기값 설정
  (Utilities|FlowControl|Sequence
    (:then_0
      (Variables|Default|SetCurState "NewEnumerator0"))
    (:then_1
      (Variables|Default|SetTargetPos (Transformation|GetActorLocation)))
    (:then_2
      (Variables|Default|SetCheckCloseTarget (* (Variables|Default|GetSpeed) 0.6)))))