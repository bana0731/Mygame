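; NPC actor that shows a dialogue box when the player (BP_MyPlayer) enters its trigger box and clears it when the player leaves.
; The construction script loads the NPC's name and lines from a fixed row of NPC_Dialog_Table into Info.
; Each entry creates a new UMG_UIE_Dialog for the DialogBox widget component, cycling through three lines via a modulo counter.
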(event OnComponentBeginOverlap(Box)
  (params (OverlappedComponent :type Primitive%20Component%20Object%20Reference) (OtherActor :type Actor%20Object%20Reference) (OtherComp :type Primitive%20Component%20Object%20Reference) (OtherBodyIndex :type Integer) (bFromSweep :type Boolean) (SweepResult :type Hit%20Result%20Structure%20%28by%20ref%29))
  (bind _info (Variables|Default|GetInfo))
  (bind (_name _script_0 _script_1 _script_2) (Utilities|Struct|BreakBPS_NPCInfo _info))
  (Utilities|Casting|CastToBP_MyPlayer OtherActor)
  (bind _returnvalue (UserInterface|CreateWidget "/Game/MY/6UMG/UMG_UIE_Dialog.UMG_UIE_Dialog_C" 0 _name (Utilities|Array|Get(acopy) (Utilities|Array|MakeArray _script_0 _script_1 _script_2) (Math|Integer|%(Integer) (Variables|Default|GetScriptIndex) 3))))
  (UserInterface|SetWidget (Variables|Default|GetDialogBox) _returnvalue)
  (Variables|Default|SetScriptIndex (+ (Variables|Default|GetScriptIndex) 1)))

(event OnComponentEndOverlap(Box)
  (params (OverlappedComponent :type Primitive%20Component%20Object%20Reference) (OtherActor :type Actor%20Object%20Reference) (OtherComp :type Primitive%20Component%20Object%20Reference) (OtherBodyIndex :type Integer))
  ;[1 1 1] 메세지창 사라짐
  (Utilities|Casting|CastToBP_MyPlayer OtherActor)
  (UserInterface|SetWidget (Variables|Default|GetDialogBox) 0))

(event EventBeginPlay)

(event Collision|EventActorBeginOverlap
  (params (OtherActor :type Actor%20Object%20Reference)))

(event EventTick
  (params (DeltaSeconds :type Float%20%28single-precision%29)))

(fn ConstructionScript
  (bind _returnvalue (Utilities|GetDataTableRow "/Game/MY/7IMG/NPC_Dialog_Table.NPC_Dialog_Table" "0")
    (:then
      (Variables|Default|SetInfo _returnvalue))))